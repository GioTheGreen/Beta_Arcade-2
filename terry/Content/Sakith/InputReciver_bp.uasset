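; InputReciver_bp receives one player's menu input for character selection and spawning.
; Outside of a match, as reported by the game mode, Menu_Enter asks it to display the selection screen if no valid character menu exists.
; With a menu open, Enter has the game mode spawn the player with the chosen character, then removes the menu.
; Menu_L and Menu_R cycle characters on that menu.
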(event Input|ActionEvents|InputActionMenu_L
  (params (Key :type Key%20Structure :default "None"))
  (bind _charectermenuref (Variables|Default|GetCharecterMenuRef))
  (:Pressed
    (Utilities|IsValid _charectermenuref
      (:Is%20Valid
        (Default|SwitchCharecter _charectermenuref -1)))))

(event Input|ActionEvents|InputActionMenu_R
  (params (Key :type Key%20Structure :default "None"))
  (bind _charectermenuref (Variables|Default|GetCharecterMenuRef))
  (:Pressed
    (Utilities|IsValid _charectermenuref
      (:Is%20Valid
        (Default|SwitchCharecter _charectermenuref 1)))))

(event Input|ActionEvents|InputActionMenu_Enter
  (params (Key :type Key%20Structure :default "None"))
  (:Pressed
    (bind _is_in_game (Class|LocalMultiplayerBpi|GetIsinGame(Message) (Game|GetGameMode)))
    (if (not _is_in_game)
      (Utilities|IsValid (Variables|Default|GetCharecterMenuRef)
        (:Is%20Valid
          (Class|LocalMultiplayerBpi|SpwanPlayer(Message) (Game|GetGameMode) (Variables|Default|GetPlayerIndex) (Variables|/Game/Sakith/UI/SakithsCS_wbp.SakithsCS_wbp_C|GetCharecterIndex (Variables|Default|GetCharecterMenuRef)) self)
          (Widget|RemovefromParent (Variables|Default|GetCharecterMenuRef))
          (Variables|Default|SetCharecterMenuRef 0))
        (:Is%20Not%20Valid
          (Class|LocalMultiplayerBpi|DisplayCS(Message) (Game|GetGameMode) (Variables|Default|GetPlayerIndex)))))))

(fn ConstructionScript)