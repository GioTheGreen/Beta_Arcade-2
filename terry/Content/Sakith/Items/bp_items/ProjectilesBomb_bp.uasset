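; Bomb item actor that, once activated, blinks as a countdown and then releases a ProjectilesSwingBomb_bp.
; The Ex timeline's Beep track is thresholded to switch the point light between its set intensity and off.
; When the timeline finishes, it spawns that follow-up actor at its own location with zero rotation and destroys itself.
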(event Custom|activate
  (bind _beep (Timeline|ex Play)
    (:Update
      (Rendering|Components|Light|SetIntensity (Variables|Default|GetPointLight) (Math|Float|SelectFloat (Variables|Default|Getintensicy) 0.0 (> _beep 0.5))))
    (:Finished
      (Game|SpawnActorfromClass "/Game/Sakith/Items/bp_items/ProjectilesSwingBomb_bp.ProjectilesSwingBomb_bp_C" (Math|Transform|MakeTransform (Transformation|GetActorLocation)) "Undefined" 0 0 0)
      (Actor|DestroyActor))))

(event EventBeginPlay
  (|CallParentFunction))

(event Collision|EventActorBeginOverlap
  (params (OtherActor :type Actor%20Object%20Reference))
  (|CallParentFunction OtherActor) ; This node is disabled and will not be called.\nDrag off pins to build functionality.
)

(event EventTick
  (params (DeltaSeconds :type Float%20%28single-precision%29))
  (|CallParentFunction DeltaSeconds) ; This node is disabled and will not be called.\nDrag off pins to build functionality.
)

(fn ConstructionScript
  (|CallParentFunction))