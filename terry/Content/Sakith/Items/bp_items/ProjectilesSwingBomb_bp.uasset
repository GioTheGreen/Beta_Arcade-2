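; ProjectilesSwingBomb is an item projectile Blueprint that provides a knockback launch for characters.
; Its Launch function normalizes the vector from the bomb's static mesh to a character's capsule and scales it by ThrowPower.
; That result supplies the horizontal velocity for LaunchCharacter, while a separate LaunchVelocityZ value sets the vertical push.
; The event graph holds only disabled default events, and nothing in this file calls Launch.
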(event EventBeginPlay
  (|CallParentFunction) ; This node is disabled and will not be called.\nDrag off pins to build functionality.
)

(event Collision|EventActorBeginOverlap
  (params (OtherActor :type Actor%20Object%20Reference))
  (|CallParentFunction OtherActor) ; This node is disabled and will not be called.\nDrag off pins to build functionality.
)

(event EventTick
  (params (DeltaSeconds :type Float%20%28single-precision%29))
  (|CallParentFunction DeltaSeconds) ; This node is disabled and will not be called.\nDrag off pins to build functionality.
)

(fn ConstructionScript
  (|CallParentFunction))

(fn Launch
  (params (A :type Object%20Object%20Reference) (self2 :type Character%20Object%20Reference) (self3 :type Character%20Object%20Reference))
  (bind _throwpower (Variables|Default|GetthrowPower))
  (bind _staticmesh (Variables|Default|GetStaticMesh))
  (bind _capsulecomponent (Variables|/Script/Engine.Character|GetCapsuleComponent self2))
  (bind _returnvalue (Transformation|GetWorldLocation _capsulecomponent))
  (bind _returnvalue_2 (Transformation|GetWorldLocation _staticmesh))
  (bind _returnvalue_3 (- _returnvalue _returnvalue_2))
  (bind _returnvalue_4 (Math|Vector|Normalize _returnvalue_3))
  (bind _returnvalue_5 (* _returnvalue_4 _throwpower))
  (Character|LaunchCharacter self3 (Math|Vector|MakeVector (.x _returnvalue_5) (.y _returnvalue_5) (Variables|Default|GetLaunch%20velocity%20z)) false false))