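; Projectile weapon item that knocks players back while in flight and can be picked up when slow or stationary.
; Box overlap launches a player away and upward if speed meets a threshold and they are not ignored; otherwise it joins their possible pickups until overlap ends.
; ResetIgnore sets the ignored player, then clears it through a timeline update.
; Construction applies scale and initial speed and sets the held object to the melee sword; Thrown is empty.
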(event OnComponentBeginOverlap(Box)
  (params (OverlappedComponent :type Primitive%20Component%20Object%20Reference) (OtherActor :type Actor%20Object%20Reference) (OtherComp :type Primitive%20Component%20Object%20Reference) (OtherBodyIndex :type Integer) (bFromSweep :type Boolean) (SweepResult :type Hit%20Result%20Structure%20%28by%20ref%29))
  (bind _assakiths_player_bp (Utilities|Casting|CastToSakithsPlayer_bp OtherActor))
  (if (and (>= (Math|Vector|VectorLength (Transformation|GetVelocity)) (Variables|Default|GetMinSationalryVelocity)) (!= _assakiths_player_bp (Variables|Default|GetIgnore)))
    (Character|LaunchCharacter _assakiths_player_bp (Math|Vector|MakeVector (.x (* (Math|Vector|Normalize (- (Transformation|GetWorldLocation (Variables|/Script/Engine.Character|GetCapsuleComponent _assakiths_player_bp)) (Transformation|GetWorldLocation (Variables|Default|GetStaticMesh)))) 5e+02)) (.y (* (Math|Vector|Normalize (- (Transformation|GetWorldLocation (Variables|/Script/Engine.Character|GetCapsuleComponent _assakiths_player_bp)) (Transformation|GetWorldLocation (Variables|Default|GetStaticMesh)))) 5e+02)) 4e+02) false false)
    (else
      (Utilities|Array|AddUnique (Variables|/Game/Sakith/SakithsPlayer_bp.SakithsPlayer_bp_C|GetPossiblePickups _assakiths_player_bp) self))))

(event OnComponentEndOverlap(Box)
  (params (OverlappedComponent :type Primitive%20Component%20Object%20Reference) (OtherActor :type Actor%20Object%20Reference) (OtherComp :type Primitive%20Component%20Object%20Reference) (OtherBodyIndex :type Integer))
  (bind _self self)
  (bind _assakiths_player_bp (Utilities|Casting|CastToSakithsPlayer_bp OtherActor))
  (if (Utilities|Array|ContainsItem (Variables|/Game/Sakith/SakithsPlayer_bp.SakithsPlayer_bp_C|GetPossiblePickups _assakiths_player_bp) _self)
    (Utilities|Array|RemoveItem (Variables|/Game/Sakith/SakithsPlayer_bp.SakithsPlayer_bp_C|GetPossiblePickups _assakiths_player_bp) _self)))

(event Custom|ResetIgnore
  (params (PlayerToIgnore :type Sakiths%20Player%20Bp%20Object%20Reference))
  ;[1 1 1] reset ignore
  (Variables|Default|SetIgnore PlayerToIgnore)
  (Timeline|reset%20ignore Play
    (:Update
      (Variables|Default|SetIgnore 0))))

(event EventBeginPlay
  (|CallParentFunction) ; This node is disabled and will not be called.\nDrag off pins to build functionality.
)

(event Collision|EventActorBeginOverlap
  (params (OtherActor :type Actor%20Object%20Reference))
  (|CallParentFunction OtherActor) ; This node is disabled and will not be called.\nDrag off pins to build functionality.
)

(event EventTick
  (params (DeltaSeconds :type Float%20%28single-precision%29))
  (|CallParentFunction DeltaSeconds))

(fn ConstructionScript
  (|CallParentFunction)
  (Variables|Default|Setheld%20object "/Game/Sakith/Items/real_Items/MeleeSwardWP_bp.MeleeSwardWP_bp_C")
  (Transformation|SetRelativeScale3D (Variables|Default|GetStaticMesh) (Variables|Default|Getscale))
  (bind _outactors (Actor|GetAllActorsOfClass "/Game/Sakith/SakithsPlayer_bp.SakithsPlayer_bp_C"))
  (Variables|Default|SetallPlayers _outactors)
  (Variables|/Script/Engine.ProjectileMovementComponent|SetInitialSpeed (Variables|Default|GetProjectileMovement) (Variables|Default|GetinialVelocity)))

(fn Thrown
  (params (owner :type Sakiths%20Player%20Bp%20Object%20Reference)))