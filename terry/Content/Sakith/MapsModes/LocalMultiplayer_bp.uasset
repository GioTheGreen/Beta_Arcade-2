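; Local multiplayer mode Blueprint that takes players from character select into a match on a shared FallowCam_bp camera.
; BeginPlay adds mode and menu widgets, creates local players in PlayerStartTag order, and has each possess an InputReciver_bp.
; DisplayCS opens character select, SpwanPlayer swaps in a SakithsPlayer_bp, and StartGame starts the camera once enough players are active.
; It also offers item lookup; Explode and Implode are stubs, and start-tag shuffling is unused.
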(event EventBeginPlay
  ;[0.2908 0.702 1] Safty check
  (bind _returnvalue (UserInterface|CreateWidget "/Game/Sakith/UI/SakithsMode_wbp.SakithsMode_wbp_C"))
  (UserInterface|Viewport|AddtoViewport _returnvalue 0)
  (bind _outactors (Actor|GetAllActorsOfClass "/Game/Sakith/FallowCam_bp.FallowCam_bp_C"))
  (Variables|Default|SetFallow_Cam (Utilities|Array|Get(acopy) _outactors))
  ;[1 1 1] Player Locations
  (CallFunction|GetPlayerStartPoints)
  (CallFunction|SpwanInputRecivers)
  (bind _returnvalue_2 (UserInterface|CreateWidget "/Game/Sakith/UI/SakithsMenu_wbp.SakithsMenu_wbp_C"))
  (bind _output_get (Variables|Default|SetMenuWbpRef _returnvalue_2))
  (UserInterface|Viewport|AddtoViewport _output_get 0))

(fn ConstructionScript)

(fn GetPlayerStartPoints
  (bind _outactors (Actor|GetAllActorsOfClass "/Script/Engine.PlayerStart"))
  (Variables|Default|SetPlayerStartArray _outactors))

(fn SpwanInputRecivers
  (for (_ _array_index) (Variables|Default|GetPlayerStartArray)
    (LocalVariables|SetIndex _array_index)
    (for (_array_element _array_index_2) (Variables|Default|GetPlayerStartArray)
      (if (== (Math|Conversions|ToInteger(Byte) (Utilities|String|ToString(Name) (Variables|/Script/Engine.PlayerStart|GetPlayerStartTag _array_element))) (LocalVariables|GetIndex))
        (Class|GameplayStatics|CreatePlayer -1)
        (bind _returnvalue (Game|SpawnActorfromClass "/Game/Sakith/InputReciver_bp.InputReciver_bp_C" (Transformation|GetActorTransform _array_element) "Undefined" 0 _array_index_2 0))
        (Utilities|Array|AddUnique (Variables|Default|GetInputRecivers) _returnvalue)
        (Pawn|Possess (Game|GetPlayerController _array_index_2) _returnvalue)
        (Utilities|Array|AddUnique (Variables|Default|GetPlayerControllers) (Game|GetPlayerController _array_index_2))
        (Game|Player|SetViewTargetwithBlend (Game|GetPlayerController _array_index_2) (Variables|Default|GetFallow_Cam) 0.0 "VTBlend_Linear" 0.0 false)))
    (CallFunction|RemoveUnusedCams)))

(fn SpawnRandomCheck
  (for (_array_element _array_index) (Variables|Default|GetPlayerStartArray)
    (for _array_element_2 (LocalVariables|GetPlayers)
      (if (== _array_element_2 (Math|Conversions|ToInteger(Byte) (Utilities|String|ToString(Name) (Variables|/Script/Engine.PlayerStart|GetPlayerStartTag _array_element))))
        (Utilities|Array|RemoveIndex (LocalVariables|GetPlayers) _array_element_2)))
    (if (== (Math|Conversions|ToInteger(Byte) (Utilities|String|ToString(Name) (Variables|/Script/Engine.PlayerStart|GetPlayerStartTag _array_element))) (Variables|Default|GetRandIndex))
      (Utilities|Array|Add (LocalVariables|Getindexes) _array_index)))
  (Utilities|Array|Shuffle (LocalVariables|GetPlayers))
  (for (_array_element_3 _array_index_2) (LocalVariables|Getindexes)
    (Variables|/Script/Engine.PlayerStart|SetPlayerStartTag (Utilities|Array|Get(acopy) (Variables|Default|GetPlayerStartArray) _array_element_3) (Utilities|String|StringToName (Utilities|String|ToString(Integer) (Utilities|Array|Get(acopy) (LocalVariables|GetPlayers) _array_index_2))))))

(fn GameStarted
  (Variables|Default|SetIsInGame true)
  (Default|GameStarted (Variables|Default|GetFallow_Cam) (Variables|Default|GetActivePlayers)))

(fn RemoveUnusedCams
  (bind _outactors (Actor|GetAllActorsOfClass "/Script/Engine.CameraActor"))
  (for _array_element _outactors
    (Actor|DestroyActor _array_element)))

(fn DisplayCS
  (params (PlayerIndex :type Integer))
  (bind _charecterselect (Default|AddCharecterSelect (Variables|Default|GetMenuWbpRef) PlayerIndex))
  (Variables|/Game/Sakith/InputReciver_bp.InputReciver_bp_C|SetCharecterMenuRef (Utilities|Array|Get(acopy) (Variables|Default|GetInputRecivers) PlayerIndex) _charecterselect)
  (return false))

(fn Explode
  (params (Power :type Float%20%28single-precision%29) (Radius :type Float%20%28single-precision%29) (StunDuration :type Float%20%28single-precision%29) (Origin :type Vector :default "0, 0, 0"))
  (return false))

(fn GetIsinGame
  (return (Variables|Default|GetIsInGame)))

(fn GetItemIndex
  (params (By%20ID? :type Boolean) (ID :type Integer) (Name :type String))
  (if By%20ID?
    (for _array_element (Variables|Default|GetItemLibary)
      (if (== (.ID (Utilities|Struct|BreakItemIndex _array_element)) ID)
        (return true _array_element)))
    (else
      (for _array_element_2 (Variables|Default|GetItemLibary)
        (if (Utilities|Enum|Equal(Enum) Name (.name (Utilities|Struct|BreakItemIndex _array_element_2)))
          (return true _array_element_2)))))
  (return false ""))

(fn Implode
  (params (Power :type Float%20%28single-precision%29) (Radius :type Float%20%28single-precision%29) (StunDuration :type Float%20%28single-precision%29) (Origin :type Vector :default "0, 0, 0"))
  (return false))

(fn SpwanPlayer
  (params (PlayerIndex :type Integer) (CharecterIndex :type Integer) (InputReciver :type Input%20Reciver%20Bp%20Object%20Reference))
  (bind _returnvalue (Game|GetPlayerController PlayerIndex))
  (bind _returnvalue_2 (Game|SpawnActorfromClass "/Game/Sakith/SakithsPlayer_bp.SakithsPlayer_bp_C" (Transformation|GetActorTransform InputReciver) "Undefined" 0 CharecterIndex 0))
  (Utilities|Array|Add (Variables|Default|GetActivePlayers) _returnvalue_2)
  (Pawn|Possess _returnvalue _returnvalue_2)
  (Game|Player|SetViewTargetwithBlend _returnvalue (Variables|Default|GetFallow_Cam) 0.0 "VTBlend_Linear" 0.0 false)
  (return false))

(fn StartGame
  (if (>= (Utilities|Array|Length (Variables|Default|GetActivePlayers)) (Variables|Default|GetMiniumPlayers))
    (CallFunction|GameStarted)
    (return false)))